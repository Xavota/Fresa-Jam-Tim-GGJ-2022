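; Test scene object that reports the active state of another object's switch through on-screen debug text.
; Every Tick it gets the Switch component from the SwitchFunc reference, reads GetActive and prints a Spanish active or inactive message.
; It has no other active logic: BeginPlay and overlap events are disabled stubs, and the construction script only calls its parent.
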(event EventBeginPlay
  (|CallParentFunction) ; This node is disabled and will not be called.\nDrag off pins to build functionality.
)

(event Collision|EventActorBeginOverlap
  (params (OtherActor :type Actor%20Object%20Reference))
  (|CallParentFunction OtherActor) ; This node is disabled and will not be called.\nDrag off pins to build functionality.
)

(event EventTick
  (params (DeltaSeconds :type Float%20%28single-precision%29))
  (|CallParentFunction DeltaSeconds)
  (bind _returnvalue (Class|Switch|GetActive (Actor|GetComponentbyClass (Variables|Default|GetSwitchFunc) "/Script/ShadowLight.Switch_C")))
  (if _returnvalue
    (Development|PrintString "El otro activo" true true "(R=0.505466,G=1.000000,B=0.000000,A=1.000000)")
    (else
      (Development|PrintString "El otro inactivo" true true "(R=0.505466,G=1.000000,B=0.000000,A=1.000000)"))))

(fn ConstructionScript
  (|CallParentFunction))