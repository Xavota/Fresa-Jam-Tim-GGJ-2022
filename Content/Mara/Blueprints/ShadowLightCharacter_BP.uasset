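; ShadowLightCharacter_BP is a character Blueprint that picks its directional walk or idle animation from movement input.
; Each Tick it reads VerticalMovement and HorizontalMovement, with vertical taking priority, and sets CurrentAnimName to a four-direction walking state.
; When movement stops, the last walking name maps to the matching idle, preserving facing.
; The name is then passed to AnimationCmp.ChangeCurrentAnimation every frame.
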(event EventBeginPlay)

(event Collision|EventActorBeginOverlap
  (params (OtherActor :type Actor%20Object%20Reference)))

(event EventTick
  (params (DeltaSeconds :type Float%20%28single-precision%29))
  (bind _verticalmovement (Variables|Default|GetVerticalMovement))
  (bind _horizontalmovement (Variables|Default|GetHorizontalMovement))
  (Utilities|FlowControl|Sequence
    (:then_0
      (if (> _verticalmovement 0.0)
        (Variables|Default|SetCurrentAnimName "WalkingUp")
        (elif (< _verticalmovement 0.0)
          (Variables|Default|SetCurrentAnimName "WalkingDown")
          (elif (> _horizontalmovement 0.0)
            (Variables|Default|SetCurrentAnimName "WalkingRight")
            (elif (< _horizontalmovement 0.0)
              (Variables|Default|SetCurrentAnimName "WalkingLeft")
              (elif (Utilities|Enum|Equal(Enum) (Variables|Default|GetCurrentAnimName) "WalkingUp")
                (Variables|Default|SetCurrentAnimName "IdleUp")
                (elif (Utilities|Enum|Equal(Enum) (Variables|Default|GetCurrentAnimName) "WalkingLeft")
                  (Variables|Default|SetCurrentAnimName "IdleLeft")
                  (elif (Utilities|Enum|Equal(Enum) (Variables|Default|GetCurrentAnimName) "WalkingRight")
                    (Variables|Default|SetCurrentAnimName "IdleRight")
                    (elif (Utilities|Enum|Equal(Enum) (Variables|Default|GetCurrentAnimName) "WalkingDown")
                      (Variables|Default|SetCurrentAnimName "IdleDown"))))))))))
    (:then_1
      (Class|Animation|ChangeCurrentAnimation (Variables|Default|GetAnimationCmp) (Variables|Default|GetCurrentAnimName)))))

(fn ConstructionScript)