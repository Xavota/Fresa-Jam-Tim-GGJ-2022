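; Test scene object enemy that cycles through a list of sprite animations to preview them in the game.
; BeginPlay initializes an animation component with the actor's sprite.
; Tick accumulates time, advances to the next animation name in a wrapping loop whenever the change interval elapses, and passes the current name to the animation component every frame.
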(event EventBeginPlay
  (|CallParentFunction)
  (Class|Animation|InitComponent (Variables|Default|GetAnimation_C) (Variables|Default|GetSprite)))

(event Collision|EventActorBeginOverlap
  (params (OtherActor :type Actor%20Object%20Reference))
  (|CallParentFunction OtherActor) ; This node is disabled and will not be called.\nDrag off pins to build functionality.
)

(event EventTick
  (params (DeltaSeconds :type Float%20%28single-precision%29))
  (|CallParentFunction DeltaSeconds)
  (Variables|Default|SetTimeElapsed (+ (Variables|Default|GetTimeElapsed) DeltaSeconds))
  (Utilities|FlowControl|Sequence
    (:then_0
      (if (>= (Variables|Default|GetTimeElapsed) (Variables|Default|GetTimeToChange))
        (bind _output_get (Variables|Default|SetCurrentAnim (Math|Integer|%(Integer) (+ (Variables|Default|GetCurrentAnim) 1) (Utilities|Array|Length (Variables|Default|GetAnimNames)))))
        (Variables|Default|SetAnimName (Utilities|Array|Get(acopy) (Variables|Default|GetAnimNames) _output_get))
        (Variables|Default|SetTimeElapsed (- (Variables|Default|GetTimeElapsed) (Variables|Default|GetTimeToChange)))))
    (:then_1
      (Class|Animation|ChangeCurrentAnimation (Variables|Default|GetAnimation_C) (Variables|Default|GetAnimName)))))

(fn ConstructionScript
  (|CallParentFunction))