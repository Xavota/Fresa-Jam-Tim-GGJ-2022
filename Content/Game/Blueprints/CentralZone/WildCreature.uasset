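; WildCreature is an actor Blueprint for a sprite-based creature in the CentralZone.
; On BeginPlay it initializes its AnimationC component with the Sprite.
; Every Tick it reads IsAlive from CreatureC and has AnimationC switch to the down-facing idle or dead animation by name.
; The construction script only calls its parent, and the overlap event is disabled.
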(event EventBeginPlay
  (|CallParentFunction)
  (Class|Animation|InitComponent (Variables|Default|GetAnimation_C) (Variables|Default|GetSprite)))

(event Collision|EventActorBeginOverlap
  (params (OtherActor :type Actor%20Object%20Reference))
  (|CallParentFunction OtherActor) ; This node is disabled and will not be called.\nDrag off pins to build functionality.
)

(event EventTick
  (params (DeltaSeconds :type Float%20%28single-precision%29))
  (bind _animation_c (Variables|Default|GetAnimation_C))
  (|CallParentFunction DeltaSeconds)
  (if (Variables|/Script/ShadowLight.Creature_C|GetIsAlive (Variables|Default|GetCreature_C))
    (Class|Animation|ChangeCurrentAnimation _animation_c "IdleDown")
    (else
      (Class|Animation|ChangeCurrentAnimation _animation_c "DeadDown"))))

(fn ConstructionScript
  (|CallParentFunction))