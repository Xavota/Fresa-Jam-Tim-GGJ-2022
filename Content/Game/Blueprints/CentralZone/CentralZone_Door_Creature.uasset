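; Central zone door that opens only when none of the creatures in its Creatures list are alive.
; Each tick it checks every listed actor's Creature component and sets the door component's pass state from the result.
; It then switches its sprite animation between Open and Closed to match, using an animation component initialised on BeginPlay.
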(event EventBeginPlay
  (|CallParentFunction)
  (Class|Animation|InitComponent (Variables|Default|GetAnimation_C) (Variables|Default|GetSprite)))

(event Collision|EventActorBeginOverlap
  (params (OtherActor :type Actor%20Object%20Reference))
  (|CallParentFunction OtherActor) ; This node is disabled and will not be called.\nDrag off pins to build functionality.
)

(event EventTick
  (params (DeltaSeconds :type Float%20%28single-precision%29))
  (|CallParentFunction DeltaSeconds)
  (Utilities|FlowControl|Sequence
    (:then_0
      (Variables|Default|SetIsOpen true)
      (for _array_element (Variables|Default|GetCreatures)
        (if (> (Utilities|Array|Length (Actor|GetComponentsByClass _array_element "/Script/ShadowLight.Creature_C")) 0)
          (if (Variables|/Script/ShadowLight.Creature_C|GetIsAlive (Utilities|Array|Get(acopy) (Actor|GetComponentsByClass _array_element "/Script/ShadowLight.Creature_C")))
            (Variables|Default|SetIsOpen false))))
      (Class|Door|SetCanPass (Variables|Default|GetDoor_C) (Variables|Default|GetIsOpen)))
    (:then_1
      (if (Variables|/Script/ShadowLight.Door_C|GetCanPass (Variables|Default|GetDoor_C))
        (Class|Animation|ChangeCurrentAnimation (Variables|Default|GetAnimation_C) "Open")
        (else
          (Class|Animation|ChangeCurrentAnimation (Variables|Default|GetAnimation_C) "Closed"))))))

(fn ConstructionScript
  (|CallParentFunction))