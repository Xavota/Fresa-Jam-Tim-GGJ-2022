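; Light2DBP is a 2D light actor that renders its light geometry and parameters every tick.
; It calls CalculateLight, clears a render target to white, then draws the Tris triangles onto it through a canvas.
; It also writes the light's world XY location and intensity into a Material Parameter Collection for materials to read.
; The triangle calculation itself is not defined in these graphs.
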(event EventBeginPlay)

(event Collision|EventActorBeginOverlap
  (params (OtherActor :type Actor%20Object%20Reference)))

(event EventTick
  (params (DeltaSeconds :type Float%20%28single-precision%29))
  (bind _texture_render_target (Variables|Default|GetTexture%20Render%20Target))
  (bind _locationworld (Variables|Default|GetlocationWorld))
  (bind (_x _y) (Math|Vector2D|BreakVector2D _locationworld))
  (Utilities|FlowControl|Sequence
    (:then_0
      (Class|Light2D|CalculateLight)
      (Rendering|ClearRenderTarget2D _texture_render_target "(R=1.000000,G=1.000000,B=1.000000,A=1.000000)")
      (bind (_canvas _size _context) (Rendering|BeginDrawCanvastoRenderTarget _texture_render_target))
      (Class|Canvas|DrawTriangle _canvas _texture_render_target (Variables|Default|Gettris))
      (Rendering|EndDrawCanvastoRenderTarget _context))
    (:then_1
      (Rendering|Material|SetVectorParameterValue "/Game/Rivaz/TwinStick/NewMaterialParameterCollection.NewMaterialParameterCollection" (Variables|Default|Getlocation) (Utilities|Struct|MakeLinearColor _x _y 0.0 0.0) :!class /Script/Engine.KismetMaterialLibrary)
      (Rendering|Material|SetScalarParameterValue "/Game/Rivaz/TwinStick/NewMaterialParameterCollection.NewMaterialParameterCollection" (Variables|Default|GetintensityName) (Variables|Default|Getintensity) :!class /Script/Engine.KismetMaterialLibrary))))

(fn ConstructionScript)